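; BP_IceMan_AIC is the AI controller for IceMan, running BP_IceMan_BT when it possesses a pawn.
; On BeginPlay it writes the player's BP_RockManCharacter to the blackboard as PlayerActor.
; Tick polls BP_RockmanGameMode for stage step changes, switching IceManBattleOn off at Stage Start and on at Stage Playing.
; SetMoveToActor stores three move target actors; the perception update event is empty.
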(event `self.ReceiveBeginPlay`
  (bind _asbp_rock_man_character (cast `/Game/Player_BP/BP_RockManCharacter` (`GameplayStatics.GetPlayerCharacter` 0)))
  (`BlackboardComponent.SetValueAsObject` (`self.Blackboard`) (`self.PlayerActor`) _asbp_rock_man_character))

(event `self.ReceivePossess`
  (params (PossessedPawn :type "Pawn Object Reference"))
  (`self.RunBehaviorTree` "/Game/BP/BP_IceMan/BP_IceMan_BT.BP_IceMan_BT"))

(event `self.ReceiveTick`
  (params (DeltaSeconds :type "Float (single-precision)"))
  (bind _blackboard (`self.Blackboard`))
  (bind _icemanbattleon (`self.IceManBattleOn`))
  (bind _asbp_rockman_game_mode (cast `/Game/BP/BP_RockmanGameMode` (`GameplayStatics.GetGameMode`))
    (:`then`
      (bind _returnvalue (`RockmanGameMode.GetNowStep` _asbp_rockman_game_mode))
      (if (!= _returnvalue (`self.StageFlow`))
        (bind _output_get (set `self.StageFlow` _returnvalue))
        (switch `EStageFlow` _output_get
          (:`stageStart`
            (`BlackboardComponent.SetValueAsBool` _blackboard _icemanbattleon false))
          (:`stagePlaying`
            (`BlackboardComponent.SetValueAsBool` _blackboard _icemanbattleon true)))))
    (:`CastFailed`
      (`KismetSystemLibrary.PrintString` "BP_Player: CastRockManGameMode error"))))

(event `self.AIPerception.OnTargetPerceptionUpdated`
  (params (Actor :type "Actor Object Reference") (Stimulus :type "AIStimulus Structure")))

(fn `SetMoveToActor`
  (params (MoveToA :type "Actor Object Reference") (MoveToB :type "Actor Object Reference") (MoveToC :type "Actor Object Reference"))
  (set `self.ActorA` MoveToA)
  (set `self.ActorB` MoveToB)
  (set `self.ActorC` MoveToC)
  (`KismetSystemLibrary.PrintString` "MoveActorSetFinished"))

(fn `UserConstructionScript`)