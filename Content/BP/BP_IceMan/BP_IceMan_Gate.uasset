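; Boss gate actor for the IceMan stage that closes segment by segment as a start sequence in the Rockman game mode.
; Tick accumulates a rate derived from MaxSpawnNum and the game mode's start time, assuming 30 fps, adding a downward-stacked paper sprite with a gate sound at each whole step.
; The last segment advances the game mode step, then again after a start-time delay.
; A construction-script prebuild with blocking collision is left unconnected.
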(event `self.ReceiveBeginPlay`
  (set `self.NowSpawnNum` 0))

(event `self.ReceiveTick`
  (params (DeltaSeconds :type "Float (single-precision)"))
  (if (< (`self.NowSpawnNum`) (`self.MaxSpawnNum`))
    (bind _asbp_rockman_game_mode (cast `/Game/BP/BP_RockmanGameMode` (`GameplayStatics.GetGameMode`)))
    (bind _output_get (set `self.StageStartAddActor` (+ (`self.StageStartAddActor`) (/ (`KismetMathLibrary.Conv_IntToDouble` (`self.MaxSpawnNum`)) (* (`RockmanGameMode.GetGameStartTime` _asbp_rockman_game_mode) 30.0)))))
    (if (> _output_get 1.0)
      (set `self.StageStartAddActor` (- (`self.StageStartAddActor`) 1.0))
      (bind _output_get_2 (set `self.NowSpawnNum` (+ (`self.NowSpawnNum`) 1)))
      (`AddComponent|NODE_AddPaperSpriteComponent-1` :`RelativeTransform` (`KismetMathLibrary.MakeTransform` (`KismetMathLibrary.MakeVector` 0.0 0.0 (* _output_get_2 -20.0))))
      (`GameplayStatics.PlaySound2D` "/Game/RockManResource/SE/BossGate.BossGate" 1.0 1.0 0.0 null null)
      (if (== (`self.MaxSpawnNum`) (`self.NowSpawnNum`))
        (bind _asbp_rockman_game_mode_2 (cast `/Game/BP/BP_RockmanGameMode` (`GameplayStatics.GetGameMode`)))
        (`RockmanGameMode.NextStep` _asbp_rockman_game_mode_2)
        (`KismetSystemLibrary.Delay` (`RockmanGameMode.GetGameStartTime` _asbp_rockman_game_mode_2))
        (`RockmanGameMode.NextStep` _asbp_rockman_game_mode_2)
        (`KismetSystemLibrary.PrintString` "InGame")))))

(fn `UserConstructionScript`)