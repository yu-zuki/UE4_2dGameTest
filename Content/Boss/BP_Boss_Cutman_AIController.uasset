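; AI controller for the Cutman boss that drives its behavior through a Behavior Tree and Blackboard.
; On BeginPlay it sets up the boss blackboard, stores the controlled pawn as self and starts the tree.
; It then writes the side-scroller player character to the blackboard and prints the component's name for debugging.
; Helper functions update the target actor and line-of-sight keys, though nothing in this file calls them.
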(event `self.ReceiveBeginPlay`
  (bind _blackboardcomponent (`self.BlackboardComponent`))
  ;[1 1 1] ビヘイビアツリーを使うための処理
  (bind _blackboardcomponent_2 (`self.UseBlackboard` "/Game/Boss/Boss_Cutman_Blackboard.Boss_Cutman_Blackboard"))
  (`BlackboardComponent.SetValueAsObject` _blackboardcomponent_2 (`self.Key_SelfActor`) (`self.K2_GetPawn`))
  (`self.RunBehaviorTree` "/Game/Boss/Boss_Cutman_BehaviorTree.Boss_Cutman_BehaviorTree")
  (bind _asbp_2dside_scroller_character (cast `/Game/Player_BP/BP_2DSideScrollerCharacter` (`GameplayStatics.GetPlayerCharacter` 0)))
  (`BlackboardComponent.SetValueAsObject` _blackboardcomponent (`self.NewVar_0`) _asbp_2dside_scroller_character)
  (`KismetSystemLibrary.PrintString` (`KismetSystemLibrary.GetDisplayName` _blackboardcomponent)))

(fn `Target Actor Name`
  (params (`Target Actor` :type "Actor Object Reference"))
  (`BlackboardComponent.SetValueAsObject` (`self.Blackboard`) (`self.TargetActor name`) `Target Actor`))

(fn `UpdateHasLineOfSightKey `
  (params (HasLineOfSight :type Boolean))
  (`BlackboardComponent.SetValueAsBool` (`self.Blackboard`) (`self.HasLineOfSightName`) HasLineOfSight))

(fn `UserConstructionScript`)