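; Cut Man boss character with flipbook animation and walk, jump, idle and shoot actions, none triggered by its own event graph.
; Tick caches its position, which Jumpcheck compares with the player's X to jump and walk when in range, otherwise just walk.
; Walk steps toward the player with swept location changes, while SelectJump jumps at random.
; Shoot spawns one cutter bullet, passing it a player-derived target and itself, then clears its ammo flag.
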(event `self.ReceiveTick`
  (params (DeltaSeconds :type "Float (single-precision)"))
  (`parent.ReceiveTick` DeltaSeconds)
  (set `self.Cut pos` (`self.K2_GetActorLocation`)))

(fn `Cut Jump`
  (if (`self.Jump_flag`)
    (`self.Jump`)
    (`PaperFlipbookComponent.SetFlipbook` (`self.Sprite`) null)
    (else
      (`self.Jump`)
      (`PaperFlipbookComponent.SetFlipbook` (`self.Sprite`) null)))
  (set `self.Jump_flag` (not (`self.Jump_flag`))))

(fn `Func`
  (if (`self.NewVar_0_0`)
    (`self.K2_SetActorRotation` (struct :`Yaw` 180.0))
    (else
      (`self.K2_SetActorRotation` (struct))))
  (set `self.NewVar_0_0` (not (`self.NewVar_0_0`))))

(fn `idle`
  (`PaperFlipbookComponent.SetFlipbook` (`self.Sprite`) null))

(fn `Jumpcheck`
  (bind _x (.x (`self.player pos`)))
  (bind _x_2 (.x (`self.player pos`)))
  ;[1 1 1] プレイヤーとの距離を判定し、ジャンプか移動か決める処理
  (bind _output_get (set `self.Jump_flag` (or (`KismetMathLibrary.InRange_FloatFloat` (.x (`self.Cut pos`)) (- _x_2 (`self.lange`)) _x_2) (`KismetMathLibrary.InRange_FloatFloat` (.x (`self.Cut pos`)) _x (+ _x (`self.lange`))))))
  (if _output_get
    (`self.Cut Jump`)
    (`self.Walk`)
    (`KismetSystemLibrary.PrintString` "true")
    (else
      (`self.Walk`)
      (`KismetSystemLibrary.PrintString` "false")))
  (set `self.Jump_flag` (not (`self.Jump_flag`))))

(fn `Select Jump`
  (bind _output_get (set `self.Jump_flag` (`KismetMathLibrary.RandomBool`)))
  (if _output_get
    (`self.Cut Jump`))
  (set `self.Jump_flag` (not (`self.Jump_flag`))))

(fn `shoot`
  (bind _returnvalue (`self.K2_GetActorLocation` (`GameplayStatics.GetPlayerCharacter` 0)))
  (if (`self.have bool`)
    (bind _returnvalue_2 (`|SpawnActorFromClass` "/Game/Boss/BP_CutmanBullet.BP_CutmanBullet_C" (`SceneComponent.K2_GetComponentToWorld` (`self.ShootPos`)) "Undefined" "OverrideRootScale" null null))
    (`PaperFlipbookComponent.SetFlipbook` (`self.Sprite`) null)
    (`/Game/Boss/BP_CutmanBullet.Set Player Pos` _returnvalue_2 (* (* (`KismetMathLibrary.Normal` _returnvalue) (1.2 0.0 1.2)) _returnvalue))
    (`/Game/Boss/BP_CutmanBullet.Set Cutman Actor` _returnvalue_2 self)
    (set `self.have bool` false)))

(fn `UserConstructionScript`
  (`parent.UserConstructionScript`))

(fn `Walk`
  (locals (NewLocalVar_0 :type "Vector Structure" :default (0.0 0.0 0.0)))
  (bind _cut_pos_x (`KismetMathLibrary.BreakVector` (`self.Cut pos`)))
  (bind _player_pos_x (`KismetMathLibrary.BreakVector` (`self.player pos`)))
  (bind _output_get (set `self.walkFlag` (>= _player_pos_x _cut_pos_x)))
  (if _output_get
    (`self.K2_SetActorLocation` (+ (`self.Cut pos`) (5.0 0.0 0.0)) true)
    (else
      (`self.K2_SetActorLocation` (+ (`self.Cut pos`) (-5.0 0.0 0.0)) true)))
  (`PaperFlipbookComponent.SetFlipbook` (`self.Sprite`) null)
  (set `self.walkFlag` (not (`self.walkFlag`))))