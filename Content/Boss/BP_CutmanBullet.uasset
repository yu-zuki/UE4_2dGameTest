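; BP_CutmanBullet is a projectile for the Cutman boss that moves toward a supplied player position.
; Setters receive that position and the Cutman actor.
; Each Tick steps it at a fixed, frame-rate-dependent speed in the XZ plane, without sweeping.
; The branch condition is hardwired true, so the alternate movement away from Cutman never runs, and no overlap or damage logic exists.
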(event `self.ReceiveTick`
  (params (DeltaSeconds :type "Float (single-precision)"))
  (bind _returnvalue (`self.K2_GetActorLocation`))
  (bind _returnvalue_2 (`self.K2_GetActorLocation`))
  (if true
    (`self.K2_SetActorLocation` (+ _returnvalue (* (`KismetMathLibrary.Normal` (- (`self.Player Pos`) _returnvalue) 5.0) (5.0 0.0 5.0))))
    (else
      (`self.K2_SetActorLocation` (+ (* (`KismetMathLibrary.Normal` (- _returnvalue_2 (`self.K2_GetActorLocation` (`self.Cutman Actor`)))) (5.0 0.0 5.0)) _returnvalue_2)))))

(fn `Set Cutman Actor`
  (params (NewParam :type "Actor Object Reference"))
  (set `self.Cutman Actor` NewParam))

(fn `Set Player Pos`
  (params (`Temp Pos` :type "Vector Structure"))
  (set `self.Player Pos` `Temp Pos`))

(fn `UserConstructionScript`)