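; Player character Blueprint for a Rockman game, handling stage-gated input, movement speed, damage sound and death.
; Input starts disabled, and each Tick polls the GameMode's step to disable it on Stage Start or enable it on Stage Playing.
; Tick also lowers walk speed while falling.
; Death opens the restart level and decrements lives stored in the GameInstance, while the HUD creation code is disconnected and never runs.
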(event `self.ReceiveBeginPlay`
  ;[1 1 1] ゲーム開始時、プレーヤー操作を無効
  (`self.DisableInput` null))

(event `self.ReceiveTick`
  (params (DeltaSeconds :type "Float (single-precision)"))
  (bind _charactermovement (`self.CharacterMovement`))
  ;[1 1 1] ゲームステップによっての処理・CPPと連携
  (`self.StageFlowProcess`)
  (if (`NavMovementComponent.IsFalling` (`self.CharacterMovement`))
    (set `CharacterMovementComponent.MaxWalkSpeed` 300.0 _charactermovement)
    (else
      (set `CharacterMovementComponent.MaxWalkSpeed` 400.0 _charactermovement))))

(event `self.IsDeath`
  ;[1 1 1] 死亡処理
  (`GameplayStatics.OpenLevel` "GameRestart_Level")
  (bind _asbp_rock_man_game_instance (cast `/Game/BP/BP_RockManGameInstance` (`GameplayStatics.GetGameInstance`)))
  (bind _returnvalue (`RockManGameInstance.getPlayerLife` _asbp_rock_man_game_instance))
  (`RockManGameInstance.setPlayerLife` _asbp_rock_man_game_instance (- _returnvalue 1)))

(event `PlayerPlaySound_1`
  (`GameplayStatics.PlaySound2D` "/Game/RockManResource/SE/RocManDamge.RocManDamge" 1.5 1.0 0.0 null null))

(fn `StageFlowProcess`
  (bind _asbp_rockman_game_mode (cast `/Game/BP/BP_RockmanGameMode` (`GameplayStatics.GetGameMode`))
    (:`then`
      (bind _returnvalue (`RockmanGameMode.GetNowStep` _asbp_rockman_game_mode))
      (if (!= _returnvalue (`self.StageFlow`))
        (bind _output_get (set `self.StageFlow` _returnvalue))
        (switch `EStageFlow` _output_get
          (:`stageStart`
            (`self.DisableInput` self null))
          (:`stagePlaying`
            (`self.EnableInput` self null)))))
    (:`CastFailed`
      (`KismetSystemLibrary.PrintString` "BP_Player: CastRockManGameMode error"))))

(fn `UserConstructionScript`)